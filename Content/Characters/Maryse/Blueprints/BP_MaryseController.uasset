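; Player controller for the Maryse character that turns movement and crouch input into actions on the controlled pawn.
; The forward and right axis events add movement input along the pawn's own forward and right vectors.
; Pressing and releasing the Crouch action casts the pawn to MaryseBlueprint and calls Crouch or UnCrouch on it.
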(event EventBeginPlay)

(event EventTick
  (params (DeltaSeconds :type Float%20%28single-precision%29)))

(event Input|ActionEvents|InputActionCrouch
  (params (Key :type Key%20Structure :default "None"))
  (bind _returnvalue (Pawn|GetControlledPawn))
  (:Pressed
    (bind _asmaryse_blueprint (Utilities|Casting|CastToMaryseBlueprint _returnvalue))
    (Character|Crouch _asmaryse_blueprint))
  (:Released
    (bind _asmaryse_blueprint_2 (Utilities|Casting|CastToMaryseBlueprint _returnvalue))
    (Character|UnCrouch _asmaryse_blueprint_2)))

(event Input|AxisEvents|InputAxisMoveForward
  (params (AxisValue :type Float%20%28single-precision%29))
  (bind _returnvalue (Pawn|GetControlledPawn))
  (Pawn|Input|AddMovementInput _returnvalue (Transformation|GetActorForwardVector _returnvalue) AxisValue false))

(event Input|AxisEvents|InputAxisMoveright
  (params (AxisValue :type Float%20%28single-precision%29))
  (bind _returnvalue (Pawn|GetControlledPawn))
  (Pawn|Input|AddMovementInput _returnvalue (Transformation|GetActorRightVector _returnvalue) AxisValue false))

(fn ConstructionScript)